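; Dialogue component for the librarian NPC "lib", who greets a new student and sends them to read books about yokai in the library.
; It extends the parent Dialogue, chaining AddDialogue calls with player options under tree index 0, the only index handled.
; All three number picks give the same errand, but only the first rewinds progress and closes, the second sets tree index 2, and the third has no follow-up.
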(fn `Dialogue`
  (`parent.Dialogue`)
  (switch `int` (`self.DialogueTreeIndex`)
    (:`0`
      (bind (_newparam _optionindex) (`self.AddDialogue` "lib" "처음 보는 얼굴인데 신입생인가요? 반가워요. 전 도서관의 사서를 맡고있는 서문채에요. " (`|MakeArray` "안녕하세요!" :!type "Text")))
      (switch `/Game/NormalChatSystem/ChatSysBP/Enum_DialogueState` _newparam
        (:`NewEnumerator0`
          (switch `int` _optionindex
            (:`0`
              (bind (_newparam_2 _optionindex_2) (`self.AddDialogue` "lib" "전훈 선생님께서 여러분들 주라고 맡기신 물건이 있는데… 그냥 주는건 별로 재미 없으니까요. 숫자 하나를 골라보세요!" (`|MakeArray` "1" "2" "3" :!type "Text")))
              (switch `/Game/NormalChatSystem/ChatSysBP/Enum_DialogueState` _newparam_2
                (:`NewEnumerator0`
                  (switch `int` _optionindex_2
                    (:`0`
                      (bind _newparam_3 (`self.AddDialogue` "lib" "1번! 요괴네요. 도서관을 돌아다니며 요괴에 대한 책을 읽고 돌아오세요."))
                      (switch `/Game/NormalChatSystem/ChatSysBP/Enum_DialogueState` _newparam_3
                        (:`NewEnumerator0`
                          (`self.RemoveDialogueProgress` 1)
                          (`self.CloseConversation`))))
                    (:`1`
                      (bind _newparam_4 (`self.AddDialogue` "lib" "2번! 요괴네요. 도서관을 돌아다니며 요괴에 대한 책을 읽고 돌아오세요."))
                      (switch `/Game/NormalChatSystem/ChatSysBP/Enum_DialogueState` _newparam_4
                        (:`NewEnumerator0`
                          (`self.SetDialogTreeIndex` 2))))
                    (:`2`
                      (`self.AddDialogue` "lib" "3번! 요괴네요. 도서관을 돌아다니며 요괴에 대한 책을 읽고 돌아오세요."))))))))))))