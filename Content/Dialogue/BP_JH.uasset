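; BP_JH is a dialogue Blueprint that shows its lines on screen one at a time through a Talk event.
; Each Talk call increments TalkIndex and, while it is at most the Dialogue array length, writes that entry into the widget's Talktext.
; The WB_Dialogue widget is created for player 0 and added to the viewport only when no valid instance exists, then reused.
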(event `/Game/Dialogue/BPI_Dialogue.Talk`
  (bind _result (`/Engine/EditorBlueprintResources/StandardMacros.IncrementInt` (`self.talk index`))
    (:`  `
      (set `self.talk index` _result)
      (if (<= (`self.talk index`) (`KismetArrayLibrary.Array_Length` (`self.dialogue`)))
        (`self.ui`
          (:`then`
            _)
          (:`else`
            (bind _returnvalue (`|CreateWidget` "/Game/Dialogue/WB_Dialogue.WB_Dialogue_C" (`GameplayStatics.GetPlayerController` 0)))
            (bind _output_get (set `self.ui` _returnvalue))
            (`UserWidget.AddToViewport` _output_get 0)))
        (`TextBlock.SetText` (`/Game/Dialogue/WB_Dialogue.talktext` (`self.ui`)) (`KismetTextLibrary.Conv_StringToText` (`|GetArrayItem` (`self.dialogue`) (`self.talk index`))))))))

(fn `UserConstructionScript`)